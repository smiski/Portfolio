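; Platformer game mode that runs the level countdown and respawns the player character.
; After a brief BeginPlay delay, it subtracts one second, then a looping one-second timer updates the player controller's timer widget and reuses that subtraction logic.
; When time runs out, it clears the timer, shows the game-over widget, pauses the game and plays an alarm.
; RespawnCharacter spawns and possesses a new character at the GameInstance's saved spawn location.
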(event Custom|StartCountdownTimer
  (CallFunction|InitialTimerSubtraction)
  (bind _returnvalue (Utilities|Time|SetTimerbyEvent (delegate Custom|CountdownTimer) 1.0 true))
  (Variables|Default|SetCountdownTimerHandle _returnvalue))

(event Custom|CountdownTimer
  (bind _asbp_player_controller (Utilities|Casting|CastToBP_PlayerController (Game|GetPlayerController 0)))
  (Default|UpdateTimerUI (Variables|/Game/Blueprints/BP_PlayerController.BP_PlayerController_C|GetWB_Timer _asbp_player_controller) (Variables|Default|GetTimerMinutes) (Variables|Default|GetTimerSeconds))
  (Variables|Default|SetTimerSeconds (- (Variables|Default|GetTimerSeconds) 1))
  (if (< (Variables|Default|GetTimerSeconds) 0)
    (if (== (Variables|Default|GetTimerMinutes) 0)
      (Utilities|Time|ClearandInvalidateTimerbyHandle (Variables|Default|GetCountdownTimerHandle))
      (bind _returnvalue (UserInterface|CreateWidget "/Game/UI/WB_GameOver.WB_GameOver_C"))
      (UserInterface|Viewport|AddtoViewport _returnvalue 0)
      (Game|SetGamePaused true)
      (Audio|SpawnSound2D (Variables|Default|GetAlarmSound) 1.0 1.0 18.0 0)
      (else
        (Variables|Default|SetTimerMinutes (- (Variables|Default|GetTimerMinutes) 1))
        (Variables|Default|SetTimerSeconds 59)))))

(event Custom|InitialTimerSubtraction
  (Variables|Default|SetTimerSeconds (- (Variables|Default|GetTimerSeconds) 1))
  (if (< (Variables|Default|GetTimerSeconds) 0)
    (if (== (Variables|Default|GetTimerMinutes) 0)
      (Utilities|Time|ClearandInvalidateTimerbyHandle (Variables|Default|GetCountdownTimerHandle))
      (bind _returnvalue (UserInterface|CreateWidget "/Game/UI/WB_GameOver.WB_GameOver_C"))
      (UserInterface|Viewport|AddtoViewport _returnvalue 0)
      (Game|SetGamePaused true)
      (Audio|SpawnSound2D (Variables|Default|GetAlarmSound) 1.0 1.0 18.0 0)
      (else
        (Variables|Default|SetTimerMinutes (- (Variables|Default|GetTimerMinutes) 1))
        (Variables|Default|SetTimerSeconds 59)))))

(event Custom|RespawnCharacter
  (bind _asbp_game_instance (Utilities|Casting|CastToBP_GameInstance (Game|GetGameInstance)))
  (bind _returnvalue (Game|SpawnActorfromClass "/Game/Blueprints/Character/BP_Character.BP_Character_C" (Math|Transform|MakeTransform (Variables|/Game/Blueprints/BP_GameInstance.BP_GameInstance_C|GetSpawnLocation _asbp_game_instance) "0, 0, 0" "1.000000,1.000000,1.000000") "Undefined" "MultiplyWithRoot" 0 0))
  (Pawn|Possess (Game|GetPlayerController 0) _returnvalue))

(event EventBeginPlay
  (Utilities|FlowControl|Delay 0.01)
  (CallFunction|StartCountdownTimer))

(fn ConstructionScript)