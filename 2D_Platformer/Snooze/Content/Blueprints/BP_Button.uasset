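; BP_Button is a one-time pickup or checkpoint actor in a platformer, triggered through its Defeat event.
; On first defeat it adds bonus seconds to the GM_Platformer timer and passes its sprite's world location to BP_GameInstance as the new spawn location.
; It then destroys itself and plays a coin sound.
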(event Custom|Defeat
  (if (not (Variables|Default|GetIsDefeated))
    (Variables|Default|SetIsDefeated true)
    (bind _asgm_platformer (Utilities|Casting|CastToGM_Platformer (Game|GetGameMode)))
    (Variables|/Game/Blueprints/GM_Platformer.GM_Platformer_C|SetTimerSeconds _asgm_platformer (+ (Variables|/Game/Blueprints/GM_Platformer.GM_Platformer_C|GetTimerSeconds _asgm_platformer) 11))
    (bind _asbp_game_instance (Utilities|Casting|CastToBP_GameInstance (Game|GetGameInstance)))
    (Default|UpdateSpawnLocation _asbp_game_instance (Transformation|GetWorldLocation (Variables|Default|GetPaperSprite)))
    (Actor|DestroyActor)
    (Audio|PlaySound2D "/Game/Audio/coin03.coin03" 1.0 1.0 0.0 0 0)))

(fn ConstructionScript)